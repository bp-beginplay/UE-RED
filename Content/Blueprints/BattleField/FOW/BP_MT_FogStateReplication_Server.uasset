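; Server-side fog-of-war state replication Blueprint for the battlefield, overriding its parent's lookups for a client's team and picked character.
; Both overrides cast the player's PlayerState to BP_BattleFieldPlayerState and return the value stored there.
; The team lookup also writes that team back through SetTeamInt.
; Event handlers are empty, and GameInstance-based lookups with parent fallbacks remain as disconnected, unused logic.
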(event EventBeginPlay)

(event Collision|EventActorBeginOverlap
  (params (OtherActor :type Actor%20Object%20Reference)))

(event EventTick
  (params (DeltaSeconds :type Float%20%28single-precision%29)))

(event EventSetPickCharacter
  (params (_Player :type Player%20Controller%20Object%20Reference)))

(fn ConstructionScript)

(fn GetClientTeamIndex
  (params (NewPlayer :type Player%20Controller%20Object%20Reference))
  (bind _asbp_battle_field_player_state (Utilities|Casting|CastToBP_BattleFieldPlayerState (Variables|/Script/Engine.Controller|GetPlayerState NewPlayer)))
  (Class|BattleFieldPlayerState|SetTeamInt _asbp_battle_field_player_state (Class|ActorInterface|GetTeam _asbp_battle_field_player_state))
  (return (Class|ActorInterface|GetTeam _asbp_battle_field_player_state)))

(fn GetClientCharacter
  (params (NewPlayer :type Player%20Controller%20Object%20Reference))
  (bind _asbp_battle_field_player_state (Utilities|Casting|CastToBP_BattleFieldPlayerState (Variables|/Script/Engine.Controller|GetPlayerState NewPlayer)))
  (return (Class|BattleFieldPlayerState|GetPickCharacter _asbp_battle_field_player_state)))