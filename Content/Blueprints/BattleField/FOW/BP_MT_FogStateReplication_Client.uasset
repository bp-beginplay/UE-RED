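; Client-side fog-of-war state replication Blueprint for the battlefield, reduced here to a lookup of a player's picked character.
; GetClientCharacter casts the given player's PlayerState to BP_BattleFieldPlayerState and returns its GetPickCharacter result.
; BeginPlay and SetPickCharacter are empty; their controller-check and pick-setting logic is disconnected, as is an older GameInstance lookup with parent fallback.
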(event EventBeginPlay)

(event EventSetPickCharacter
  (params (_Player :type Player%20Controller%20Object%20Reference)))

(fn ConstructionScript)

(fn GetClientCharacter
  (params (NewPlayer :type Player%20Controller%20Object%20Reference))
  (bind _asbp_battle_field_player_state (Utilities|Casting|CastToBP_BattleFieldPlayerState (Variables|/Script/Engine.Controller|GetPlayerState NewPlayer)))
  (return (Class|BattleFieldPlayerState|GetPickCharacter _asbp_battle_field_player_state)))