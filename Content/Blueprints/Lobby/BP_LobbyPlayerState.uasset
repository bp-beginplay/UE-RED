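; Lobby PlayerState that relays team assignments and character picks to BP_RED_GameInstance, keyed by each player's unique net ID.
; Each Server_ event forwards its arguments to a matching Mul_ event, a server-to-multicast relay by naming.
; The Mul_ events cast the local GameInstance and call AddPlayer or SetPickCharacter, so the PlayerState stores none of this data itself.
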(event Custom|Mul_AddPlayerToTeam
  (params (Unique%20Net%20ID :type Unique%20Net%20Id%20Repl%20Structure) (Team%20Idx :type Integer))
  (bind _asbp_red_game_instance (Utilities|Casting|CastToBP_RED_GameInstance (Game|GetGameInstance)))
  (Class|RedGameInstance|AddPlayer _asbp_red_game_instance Unique%20Net%20ID Team%20Idx))

(event Custom|Server_AddPlayerToTeam
  (params (Unique%20Net%20ID :type Unique%20Net%20Id%20Repl%20Structure) (Team%20Idx :type Integer))
  (CallFunction|MulAddPlayertoTeam Unique%20Net%20ID Team%20Idx))

(event Custom|Server_SetPickCharacter
  (params (Unique%20Net%20ID :type Unique%20Net%20Id%20Repl%20Structure) (Pick%20Charater :type Name))
  (CallFunction|MulSetPickCharacter Unique%20Net%20ID Pick%20Charater))

(event Custom|Mul_SetPickCharacter
  (params (Unique%20Net%20ID :type Unique%20Net%20Id%20Repl%20Structure) (Pick%20Charater :type Name))
  (bind _asbp_red_game_instance (Utilities|Casting|CastToBP_RED_GameInstance (Game|GetGameInstance)))
  (Class|RedGameInstance|SetPickCharacter _asbp_red_game_instance Unique%20Net%20ID Pick%20Charater))

(event EventBeginPlay)

(event EventTick
  (params (DeltaSeconds :type Float%20%28single-precision%29)))

(fn ConstructionScript)